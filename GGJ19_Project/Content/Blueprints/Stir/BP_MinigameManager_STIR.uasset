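; BP_MinigameManager_STIR manages the stir minigame, hiding the spoon and stirable actor until its start event fires.
; StartEvent reveals both, waits briefly, activates the Stirable, then plays a timeline that offsets the spoon mesh from its starting relative location.
; A disconnected branch that would activate Spicies and join the same spoon animation never runs.
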(event `self.ReceiveBeginPlay`
  (`SceneComponent.SetHiddenInGame` (`self.SpoonHolder`) true true)
  (`self.SetActorHiddenInGame` (`self.Stirable`) true))

(event `StartEvent`
  (bind _stirable (`self.Stirable`))
  (bind _sm_spoon (`self.SM_Spoon`))
  (`KismetSystemLibrary.PrintString` "PhaseCook")
  (`SceneComponent.SetHiddenInGame` (`self.SM_Spoon`) false true)
  (`self.SetActorHiddenInGame` _stirable false)
  (`KismetSystemLibrary.Delay` 2.0)
  (`/Game/Blueprints/Stir/BP_Stirable.Activate` _stirable)
  (set `self.Tooltip` (`self.Tooltip`))
  (set `self.InitialLocation` (`SceneComponent.RelativeLocation` _sm_spoon))
  (bind (_direction _newtrack_0) (`Timeline|Timeline_0`)
    (:`Update`
      (`SceneComponent.K2_SetRelativeLocation` _sm_spoon (+ _newtrack_0 (`self.InitialLocation`)) false false))))

(fn `UserConstructionScript`)