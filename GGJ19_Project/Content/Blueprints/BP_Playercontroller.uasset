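; Player controller Blueprint that handles cursor, menu input and cook phase advancement.
; On BeginPlay it shows the mouse cursor on player controller 0.
; The Pause action passes the inverse of the current paused state to the HUD's paused message, and a GameOverTest action shows a test game-over message.
; A NextPhase event forwards to NextCookPhase, while Tick and the construction script do nothing.
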(event `self.ReceiveBeginPlay`
  (set `PlayerController.bShowMouseCursor` true (`GameplayStatics.GetPlayerController` 0)))

(event `InputAction|Pause`
  (params (Key :type "Key Structure"))
  ;[1 1 1] Menus
  (:`Pressed`
    (message `/Game/GameJamKit/Blueprints/BP_GameJamKit_HUD_Interface.SetPaused` (`self.GetHUD`) (not (`GameplayStatics.IsGamePaused`)))))

(event `InputAction|GameOverTest`
  (params (Key :type "Key Structure"))
  ;[1 1 1] Menus
  (:`Pressed`
    (message `/Game/GameJamKit/Blueprints/BP_GameJamKit_HUD_Interface.ShowGameOver` (`self.GetHUD`) "Game  over test")))

(event `NextPhase`
  (`self.NextCookPhase`))

(fn `UserConstructionScript`)