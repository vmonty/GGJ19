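; Cuttable actor for a cutting phase, using a procedural mesh copied from its static mesh at construction and on Activate.
; An overlap on that mesh slices it through a DoOnce gate, at the overlapping component's location along a fixed Y-normal plane with red caps.
; Each cut-off half is stored and simulates physics, and reaching MaxCuts calls EndPhase1 on the manager passed to Activate.
; ChangeVisibility toggles the actor's components via FlipFlop.
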(event `Activate`
  (params (Manager :type "/Game/Blueprints/Cut/BP_MinigameManager_CUT Object Reference"))
  ;[1 1 1] Activate: manage proc mesh and visibility
  (set `self.ManagerRef` Manager)
  (`KismetProceduralMeshLibrary.CopyProceduralMeshFromStaticMeshComponent` (`self.StaticMesh`) 0 (`self.ProceduralMesh`) true)
  (`self.SetActorHiddenInGame` false)
  (set `self.Count` 0))

(event `Reset`
  ;[1 1 1] Slice
  (goto _label :!via `Reset`))

(event `self.ProceduralMesh.OnComponentBeginOverlap`
  (params (OverlappedComponent :type "PrimitiveComponent Object Reference") (OtherActor :type "Actor Object Reference") (OtherComp :type "PrimitiveComponent Object Reference") (OtherBodyIndex :type Integer) (bFromSweep :type Boolean) (SweepResult :type "HitResult Structure (by ref)"))
  ;[1 1 1] Slice
  (`/Engine/EditorBlueprintResources/StandardMacros.DoOnce` false :!label _label
    (:`Completed`
      (`KismetSystemLibrary.PrintString` "Cut!" true true (struct :`G` 0.66 :`B` 1.0 :`A` 1.0) 60.0)
      (bind _outotherhalfprocmesh (`KismetProceduralMeshLibrary.SliceProceduralMesh` (`self.ProceduralMesh`) (`SceneComponent.K2_GetComponentLocation` OtherComp) (0.0 1.0 0.0) true "CreateNewSectionForCap" "/Game/Materials/Basic/MI_Red.MI_Red"))
      (bind _output_get (set `self.SlicedProcMesh` _outotherhalfprocmesh))
      (`KismetArrayLibrary.Array_Add` (`self.SlicesArr`) _output_get)
      (`PrimitiveComponent.SetSimulatePhysics` _output_get true)
      (`KismetSystemLibrary.PrintString` "Cut" true true (struct :`G` 0.66 :`B` 1.0 :`A` 1.0) 60.0)
      (bind _output_get_2 (set `self.Count` (+ (`self.Count`) 1)))
      (if (>= _output_get_2 (`self.MaxCuts`))
        (`/Game/Blueprints/Cut/BP_MinigameManager_CUT.EndPhase1` (`self.ManagerRef`)))
      (`self.Reset`))))

(fn `ChangeVisibility`
  (bind _defaultsceneroot (`self.DefaultSceneRoot`))
  (`/Engine/EditorBlueprintResources/StandardMacros.FlipFlop`
    (:`A`
      (`SceneComponent.SetHiddenInGame` _defaultsceneroot false true))
    (:`B`
      (`SceneComponent.SetHiddenInGame` _defaultsceneroot true true))))

(fn `UserConstructionScript`
  ;[1 1 1] Create procedural mesh
  (`KismetProceduralMeshLibrary.CopyProceduralMeshFromStaticMeshComponent` (`self.StaticMesh`) 0 (`self.ProceduralMesh`) true))