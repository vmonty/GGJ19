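; BP_Selector is an actor that lets the player pick one of two food items with the mouse for a cutting subphase.
; A manager activates it, enabling input and showing the cursor.
; Each tick, a short trace from the cursor sets the active item and highlights it through custom depth.
; Pressing Cut on an item hides the cursor and selector, then passes the choice to the manager's SubphaseCut.
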(event `self.ReceiveBeginPlay`)

(event `Activate`
  (params (Manager :type "/Game/Blueprints/Cut/BP_MinigameManager_CUT Object Reference"))
  (set `self.ManagerRef` Manager)
  (set `PlayerController.bShowMouseCursor` true (`GameplayStatics.GetPlayerController` 0))
  (`self.EnableInput` (`GameplayStatics.GetPlayerController` 0)))

(event `self.ReceiveTick`
  (params (DeltaSeconds :type "Float (single-precision)"))
  (bind _food1 (`self.Food1`))
  (bind _food2 (`self.Food2`))
  (bind (_worldlocation _worlddirection) (`PlayerController.DeprojectMousePositionToWorld` (`GameplayStatics.GetPlayerController` 0)))
  (bind _outhit (`KismetSystemLibrary.LineTraceSingle` :`Start` _worldlocation :`End` (+ _worldlocation (* _worlddirection 200.0)) :`TraceChannel` "TraceTypeQuery1" :`bIgnoreSelf` false :`DrawTime` 60.0))
  (bind (_bblockinghit _binitialoverlap _time _distance _location _impactpoint _normal _impactnormal _physmat _hitactor _hitcomponent) (`GameplayStatics.BreakHitResult` _outhit))
  (if (== _hitcomponent (`self.Food1`))
    ;[1 1 1] Manage outlines and active item
    (`PrimitiveComponent.SetRenderCustomDepth` _food1 true)
    (`PrimitiveComponent.SetRenderCustomDepth` _food2 false)
    (set `self.EnumActiveItem` "NewEnumerator1")
    (elif (== _hitcomponent (`self.Food2`))
      (`PrimitiveComponent.SetRenderCustomDepth` _food1 false)
      (`PrimitiveComponent.SetRenderCustomDepth` _food2 true)
      (set `self.EnumActiveItem` "NewEnumerator2")
      (else
        (`PrimitiveComponent.SetRenderCustomDepth` _food1 false)
        (`PrimitiveComponent.SetRenderCustomDepth` _food2 false)
        (set `self.EnumActiveItem` "NewEnumerator0")))))

(event `InputAction|Cut`
  (params (Key :type "Key Structure"))
  (:`Pressed`
    (if (`|EnumInequality` (`self.EnumActiveItem`) "NewEnumerator0")
      ;[1 1 1] Item selected: hide mouse
      (`KismetSystemLibrary.PrintString` "Item selected")
      (set `PlayerController.bShowMouseCursor` false (`GameplayStatics.GetPlayerController` 0))
      (`/Game/Blueprints/Cut/BP_MinigameManager_CUT.SubphaseCut` (`self.ManagerRef`) (`self.EnumActiveItem`))
      (`self.SetActorHiddenInGame` true))))

(fn `SwapActive`)

(fn `UserConstructionScript`)