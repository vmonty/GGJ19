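; Manager for the cutting minigame, covering dish selection and knife chopping as one cooking phase.
; BeginPlay activates the Selector; SubphaseCut then spawns a crab or lobster cuttable, records the dish in GM_GGJ and shows the knife.
; The Turn axis slides the knife sideways, and Cut plays a gated timeline chop that ends by resetting the cuttable.
; EndPhase1 advances the player controller's cook phase and removes the cuttable and knife.
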(event `self.ReceiveBeginPlay`
  (`SceneComponent.SetHiddenInGame` (`self.KnifeHolder`) true true)
  (`/Game/Blueprints/Cut/BP_Selector.Activate` (`self.Selector`) self))

(event `InputAxis|Turn` :overrideparent false
  (params (AxisValue :type "Float (single-precision)"))
  (bind _knifeholder (`self.KnifeHolder`))
  (bind (_relativelocation_x _relativelocation_y _relativelocation_z) (`KismetMathLibrary.BreakVector` (`SceneComponent.RelativeLocation` _knifeholder)))
  ;[1 1 1] Input
  ;;[1 1 1] Move the knife
  (if (not (`self.finishCutting`))
    (`SceneComponent.K2_SetRelativeLocation` _knifeholder (`KismetMathLibrary.MakeVector` _relativelocation_x (+ AxisValue _relativelocation_y) _relativelocation_z) false false)))

(event `SubphaseCut`
  (params (Enum :type "/Game/Blueprints/Cut/ENUM_Selection Enum" :default "NewEnumerator0"))
  (bind _returnvalue (`self.GetTransform` (`self.TargetLocation`)))
  (bind _asgm_ggj (cast `/Game/Blueprints/GM_GGJ` (`GameplayStatics.GetGameMode`)))
  (switch `/Game/Blueprints/Cut/ENUM_Selection` Enum
    (:`NewEnumerator1`
      (bind _returnvalue_2 (`|SpawnActorFromClass` "/Game/Blueprints/Cut/BP_Cut2_Crab.BP_Cut2_Crab_C" _returnvalue "AlwaysSpawn" "OverrideRootScale" null null))
      (set `self.Cutable1` _returnvalue_2)
      (`KitchenGameMode.SetDishChosen` _asgm_ggj "Crab"))
    (:`NewEnumerator2`
      (bind _returnvalue_3 (`|SpawnActorFromClass` "/Game/Blueprints/Cut/BP_Cut1_Lobster.BP_Cut1_Lobster_C" _returnvalue "AlwaysSpawn" "OverrideRootScale" null null))
      (set `self.Cutable1` _returnvalue_3)
      (`KitchenGameMode.SetDishChosen` _asgm_ggj "Lobster")))
  (set `self.finishCutting` false)
  (`/Game/Blueprints/Cut/BP_Cutable.Activate` (`self.Cutable1`) self)
  (`self.EnableInput` (`GameplayStatics.GetPlayerController` 0))
  (set `self.KnifeLocation` (`SceneComponent.RelativeLocation` (`self.KnifeHolder`)))
  (`SceneComponent.SetHiddenInGame` (`self.KnifeHolder`) false true))

(event `InputAction|Cut`
  (params (Key :type "Key Structure"))
  (bind _returnvalue (`GameplayStatics.GetPlayerController` 0))
  (bind (_knifelocation_x _knifelocation_y _knifelocation_z) (`KismetMathLibrary.BreakVector` (`self.KnifeLocation`)))
  (bind (_relativelocation_x _relativelocation_y) (`KismetMathLibrary.BreakVector` (`SceneComponent.RelativeLocation` (`self.KnifeHolder`))))
  (:`Pressed`
    ;[1 1 1] Input
    ;;[1 1 1] Cut input
    (if (not (`self.finishCutting`))
      (`/Engine/EditorBlueprintResources/StandardMacros.DoOnce` false :!label _label
        (:`Completed`
          (`self.DisableInput` _returnvalue)
          (bind (_direction _cut) (`Timeline|Timeline_0` :!via `PlayFromStart` :!label _label_2)
            (:`Update`
              (`SceneComponent.K2_SetRelativeLocation` (`self.KnifeHolder`) (`KismetMathLibrary.MakeVector` _relativelocation_x _relativelocation_y (- _knifelocation_z (* _knifelocation_z _cut))) false false))
            (:`Finished`
              (`/Game/Blueprints/Cut/BP_Cutable.ResetCut` (`self.Cutable1`))
              (`self.EnableInput` _returnvalue)
              (goto _label :!via `Reset`))))))))

(event `Stop`
  ;[1 1 1] Input
  ;;[1 1 1] Cut input
  (goto _label_2 :!via `Stop`))

(event `EndPhase1`
  ;[1 1 1] Manage: Select item - Cut tiem a number of times - end phsae
  (if (not (`self.finishCutting`))
    (`/Engine/EditorBlueprintResources/StandardMacros.DoOnce` false
      (:`Completed`
        (bind _asbp_playercontroller (cast `/Game/Blueprints/BP_Playercontroller` (`GameplayStatics.GetPlayerController` 0)))
        (`KitchenPlayerController.NextCookPhase` _asbp_playercontroller)
        (`KitchenPlayerController.OnPhaseChanged` _asbp_playercontroller)
        (`KismetSystemLibrary.Delay` 0.2)
        (set `self.finishCutting` true)
        (`self.Stop`)
        (`self.K2_DestroyActor` (`self.Cutable1`))
        (`ActorComponent.K2_DestroyComponent` (`self.KnifeHolder`))))))

(fn `UserConstructionScript`)