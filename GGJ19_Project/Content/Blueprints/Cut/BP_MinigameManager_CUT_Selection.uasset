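; Manager actor for the food selection step of a cutting minigame, still at a debug stage.
; BeginPlay enables input and the mouse cursor.
; The Cut action line-traces a short distance from the cursor and compares the hit actor to two food collision actors, only printing which was clicked or a miss.
; CreateOutline can add a static mesh component at Food1's transform, while SubphaseCut is an empty stub.
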(event `self.ReceiveBeginPlay`
  (`self.EnableInput` (`GameplayStatics.GetPlayerController` 0))
  (set `PlayerController.bShowMouseCursor` true (`GameplayStatics.GetPlayerController` 0)))

(event `CreateOutline`
  (if (`self.hasOutline`)
    (bind _returnvalue (`AddComponent|NODE_AddStaticMeshComponent-0` :`RelativeTransform` (`SceneComponent.K2_GetComponentToWorld` (`self.Food1`))))
    (bind _output_get (set `self.MeshComponent` _returnvalue))
    (`StaticMeshComponent.SetStaticMesh` _output_get (`self.Mesh`))))

(event `SubphaseCut`)

(event `self.ReceiveTick`
  (params (DeltaSeconds :type "Float (single-precision)")))

(event `InputAction|Cut`
  (params (Key :type "Key Structure"))
  (bind (_worldlocation _worlddirection) (`PlayerController.DeprojectMousePositionToWorld` (`GameplayStatics.GetPlayerController` 0)))
  (bind _returnvalue (+ _worldlocation (* _worlddirection 400.0)))
  (:`Pressed`
    (`KismetSystemLibrary.PrintString` (`KismetStringLibrary.Conv_VectorToString` _worldlocation))
    (`KismetSystemLibrary.PrintString` (`KismetStringLibrary.Conv_VectorToString` _returnvalue))
    (bind _outhit (`KismetSystemLibrary.LineTraceSingle` :`Start` _worldlocation :`End` _returnvalue :`TraceChannel` "TraceTypeQuery1" :`DrawDebugType` "ForDuration" :`DrawTime` 60.0))
    (bind (_bblockinghit _binitialoverlap _time _distance _location _impactpoint _normal _impactnormal _physmat _hitactor) (`GameplayStatics.BreakHitResult` _outhit))
    (`KismetSystemLibrary.PrintString` (`KismetSystemLibrary.GetDisplayName` _hitactor))
    (if (== _hitactor (`self.Food1Collision`))
      (`KismetSystemLibrary.PrintString` "Food1")
      (elif (== _hitactor (`self.Food2Collision`))
        (`KismetSystemLibrary.PrintString` "Food2")
        (else
          (`KismetSystemLibrary.PrintString` "Fail click"))))))

(fn `UserConstructionScript`)