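; Spices Blueprint that plays a scripted animation on its Spices component when Activate fires.
; Three timelines run in sequence: a relative move, a roll rotation that sets pitch and yaw to zero, then a second move from where the first ended.
; Starting location and rotation are cached on activation and restored instantly when the last timeline finishes.
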(event `Activate`
  (set `self.InitialLocation` (`SceneComponent.RelativeLocation` (`self.Spices`)))
  (set `self.InitialRotation` (`SceneComponent.RelativeRotation` (`self.Spices`)))
  (bind (_direction _newtrack_0) (`Timeline|Timeline`)
    (:`Update`
      (bind _returnvalue (+ _newtrack_0 (`self.InitialLocation`)))
      (`SceneComponent.K2_SetRelativeLocation` (`self.Spices`) _returnvalue false false)
      (set `self.SecondLocation` _returnvalue))
    (:`Finished`
      (bind (_direction_2 _newtrack_0_2) (`Timeline|Timeline1`)
        (:`Update`
          (`SceneComponent.K2_SetRelativeRotation` (`self.Spices`) (`KismetMathLibrary.MakeRotator` (+ (.roll (`self.InitialRotation`)) _newtrack_0_2)) false false))
        (:`Finished`
          (bind (_direction_3 _newtrack_0_3) (`Timeline|Timeline2`)
            (:`Update`
              (`SceneComponent.K2_SetRelativeLocation` (`self.Spices`) (+ (`self.SecondLocation`) _newtrack_0_3) false false))
            (:`Finished`
              (`SceneComponent.K2_SetRelativeLocation` (`self.Spices`) (`self.InitialLocation`) false false)
              (`SceneComponent.K2_SetRelativeRotation` (`self.Spices`) (`self.InitialRotation`) false false))))))))

(fn `UserConstructionScript`)