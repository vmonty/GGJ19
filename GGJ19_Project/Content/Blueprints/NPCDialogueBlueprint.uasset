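; NPC dialogue actor prototype that, on BeginPlay, steps through the indices of the R1Options1 string array on a timer.
; A custom Modified For Loop macro exits through Delay Out and resumes via Delay In, allowing a two-second Delay before each iteration.
; Each iteration prints only the index as a long-lasting debug string.
; Random-element sentence building and a Recipe1 loop are present but unused.
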(event `self.ReceiveBeginPlay`
  (bind _index (`self.Modified For Loop` 0 (- (`KismetArrayLibrary.Array_Length` (`self.R1Options1`)) 1) :!label _label)
    (:`LoopBody`
      (`KismetSystemLibrary.PrintString` (`KismetStringLibrary.Conv_IntToString` _index) true true (struct :`G` 0.66 :`B` 1.0 :`A` 1.0) 100.0))
    (:`DelayOut`
      (`KismetSystemLibrary.Delay` 2.0)
      (goto _label :!via `DelayIn`))))

(fn `UserConstructionScript`)