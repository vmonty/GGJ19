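; Seasoning minigame for the cooking sequence, run as Phase 2, where salt-and-pepper or paprika is chosen.
; ActivatePhase2 turns on the selector, and Subphase records the choice in GM_GGJ and spawns a Spices actor at a target point.
; A timeline animates that actor by offsetting it from its spawn location.
; When it finishes, EndPhase2 advances the player controller's cook phase and destroys the spice actor.
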(event `ActivatePhase2`
  ;[1 1 1] Activate cutted mesh; activate selectors
  (`KismetSystemLibrary.PrintString` "Phase2Started")
  (`/Game/Blueprints/Seaoned/BP_SelectorPH2.Activate` (`self.SelectorPh2`) self))

(event `Subphase`
  (params (Enum :type "/Game/Blueprints/Cut/ENUM_Selection Enum" :default "NewEnumerator0"))
  (bind _returnvalue (`self.GetTransform` (`self.TargetPoint`)))
  (bind _asgm_ggj (cast `/Game/Blueprints/GM_GGJ` (`GameplayStatics.GetGameMode`)))
  (switch `/Game/Blueprints/Cut/ENUM_Selection` Enum
    (:`NewEnumerator0`
      (`KismetSystemLibrary.PrintString` "No Season"))
    (:`NewEnumerator1`
      (`KitchenGameMode.SetSeasonChosen` _asgm_ggj "SaltPepper")
      (bind _returnvalue_2 (`|SpawnActorFromClass` "/Game/Blueprints/Spices.Spices_C" _returnvalue "AlwaysSpawn" "OverrideRootScale" null null))
      (set `self.SeasonObject` _returnvalue_2)
      (set `self.InitialLocation` (`self.K2_GetActorLocation` (`self.SeasonObject`)) :!label _label)
      (bind (_direction _newtrack_0) (`Timeline|Timeline_0`)
        (:`Update`
          (`self.K2_SetActorRelativeLocation` (`self.SeasonObject`) (+ _newtrack_0 (`self.InitialLocation`)) false false))
        (:`Finished`
          (`self.EndPhase2`))))
    (:`NewEnumerator2`
      (`KitchenGameMode.SetSeasonChosen` _asgm_ggj "Paprika")
      (bind _returnvalue_3 (`|SpawnActorFromClass` "/Game/Blueprints/Spices.Spices_C" _returnvalue "AlwaysSpawn" "OverrideRootScale" null null))
      (set `self.SeasonObject` _returnvalue_3)
      (goto _label))))

(event `EndPhase2`
  ;[1 1 1] End phase
  (`KismetSystemLibrary.PrintString` "End Seasoning!!!")
  (bind _asbp_playercontroller (cast `/Game/Blueprints/BP_Playercontroller` (`GameplayStatics.GetPlayerController` 0)))
  (`KitchenPlayerController.NextCookPhase` _asbp_playercontroller)
  (`KitchenPlayerController.OnPhaseChanged` _asbp_playercontroller)
  (`self.K2_DestroyActor` (`self.SeasonObject`)))

(fn `UserConstructionScript`)